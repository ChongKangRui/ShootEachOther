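; Gameplay ability that reloads the equipped weapon, moving rounds from spare ammo into the magazine.
; It plays the weapon's reload montage, ends with it, and transfers ammo on the Weapon.Reloaded event, capped by magazine space and remaining spare.
; An empty magazine adds a non-replicated Weapon.BlockFire tag until the ability ends.
; With no spare ammo, it adds that tag and ends immediately, leaving fire blocked.
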(event Ability|EventActivateAbility
  (bind _returnvalue (Class|SEOGameplayAbility|GetEquippedWeaponInstance))
  (Utilities|FlowControl|Sequence
    (:then_0
      (if (<= (Class|WeaponInstance|GetStatCount _returnvalue "(TagName=\"Weapon.Ammo.CurrentSpare\")") 0)
        (CallFunction|AddBlockFire)
        (Variables|Default|SetCancelBlockedFiredWhenEndAbility false)
        (Ability|EndAbility :!label _label)
        (else
          (if (<= (Class|WeaponInstance|GetStatCount _returnvalue "(TagName=\"Weapon.Ammo.Current\")") 0)
            (Variables|Default|SetCancelBlockedFiredWhenEndAbility true)
            (Ability|GameplayEffect|AddLooseGameplayTags (Ability|GetAvatarActorfromActorInfo) (GameplayTags|MakeLiteralGameplayTagContainer "(GameplayTags=((TagName=\"Weapon.BlockFire\")))")))
          (|PlayMontageandWaitProxy "None" (Utilities|Struct|BreakWeaponData (Class|WeaponInstance|GetDefaultsWeaponData (Class|SEOGameplayAbility|GetEquippedWeaponInstance))) 1.0 "None" true 1.0 0.0 false
            (:then
              (Ability|Tasks|WaitGameplayEvent "(TagName=\"Weapon.Reloaded\")" (Ability|GetAvatarActorfromActorInfo) true
                (:EventReceived
                  (CallFunction|ReloadAmmoState)
                  (Development|PrintString "Reload Completed"))))
            (:OnCompleted
              (goto _label))
            (:OnBlendOut
              (goto _label))
            (:OnInterrupted
              (goto _label))
            (:OnCancelled
              (goto _label))))))))

(event Ability|EventOnEndAbility
  (params (bWasCancelled :type Boolean))
  (if (Variables|Default|GetCancelBlockedFiredWhenEndAbility)
    (CallFunction|RemoveBlockFire)))

(fn ReloadAmmoState
  (bind _output_get (LocalVariables|SetWeaponInstance (Class|SEOGameplayAbility|GetEquippedWeaponInstance)))
  (for _array_element (.StackValue (Utilities|Struct|BreakWeaponData (Class|WeaponInstance|GetDefaultsWeaponData _output_get)))
    (|SwitchGameplayTag (.Tag (Utilities|Struct|BreakStackValue _array_element))
      (:Weapon.Ammo.Current
        (LocalVariables|SetWeaponCurrentAmmoSize (.Value (Utilities|Struct|BreakStackValue _array_element))))
      (:Weapon.Ammo.CurrentSpare
        (LocalVariables|SetWeaponSpareAmmoSize (.Value (Utilities|Struct|BreakStackValue _array_element))))))
  (LocalVariables|SetCurrentAmmo (Class|WeaponInstance|GetStatCount (LocalVariables|GetWeaponInstance) "(TagName=\"Weapon.Ammo.Current\")"))
  (LocalVariables|SetCurrentSpareAmmo (Class|WeaponInstance|GetStatCount (LocalVariables|GetWeaponInstance) "(TagName=\"Weapon.Ammo.CurrentSpare\")"))
  (Class|WeaponInstance|AddStatCount (LocalVariables|GetWeaponInstance) "(TagName=\"Weapon.Ammo.Current\")" (Math|Integer|SelectInt (LocalVariables|GetCurrentSpareAmmo) (- (LocalVariables|GetWeaponCurrentAmmoSize) (LocalVariables|GetCurrentAmmo)) (< (LocalVariables|GetCurrentSpareAmmo) (- (LocalVariables|GetWeaponCurrentAmmoSize) (LocalVariables|GetCurrentAmmo)))))
  (Class|WeaponInstance|RemoveStatCount (LocalVariables|GetWeaponInstance) "(TagName=\"Weapon.Ammo.CurrentSpare\")" (Math|Integer|SelectInt (LocalVariables|GetCurrentSpareAmmo) (- (LocalVariables|GetWeaponCurrentAmmoSize) (LocalVariables|GetCurrentAmmo)) (< (LocalVariables|GetCurrentSpareAmmo) (- (LocalVariables|GetWeaponCurrentAmmoSize) (LocalVariables|GetCurrentAmmo))))))

(fn AddBlockFire
  (bind _returnvalue (Ability|GetOwningActorfromActorInfo))
  (Ability|GameplayEffect|AddLooseGameplayTags _returnvalue (GameplayTags|MakeLiteralGameplayTagContainer "(GameplayTags=((TagName=\"Weapon.BlockFire\")))"))
  (Development|PrintString (Utilities|GetDisplayName _returnvalue)))

(fn RemoveBlockFire
  (Ability|GameplayEffect|RemoveLooseGameplayTags (Ability|GetOwningActorfromActorInfo) (GameplayTags|MakeLiteralGameplayTagContainer "(GameplayTags=((TagName=\"Weapon.BlockFire\")))")))