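; GA_Death is the Gameplay Ability that handles a character's death for BP_FirstPersonCharacter.
; On activation it stops the bot controller's brain logic if the owner's player state is a bot, then starts server-side ragdoll on the character.
; It finally adds a replicated loose Gameplay.AbilityInputBlocked tag to the ability system owner; the graph never ends the ability.
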(event Ability|EventActivateAbility
  (bind _asbp_first_person_character (Utilities|Casting|CastToBP_FirstPersonCharacter (Class|SEOGameplayAbility|GetSEOCharacter)))
  (if (Variables|/Script/Engine.PlayerState|GetbIsABot (Class|ShootEachOtherCharacter|GetSEOPlayerState _asbp_first_person_character))
    (AI|Logic|StopLogic (Variables|/Script/AIModule.AIController|GetBrainComponent (Class|ShootEachOtherCharacter|GetBotController _asbp_first_person_character)) "Death"))
  (Default|StartRagdollServer _asbp_first_person_character)
  (Ability|GameplayEffect|AddLooseGameplayTags (Components|GetOwner (Class|SEOGameplayAbility|GetSEOAbilitySystemComponent)) (GameplayTags|MakeLiteralGameplayTagContainer "(GameplayTags=((TagName=\"Gameplay.AbilityInputBlocked\")))") true))

(event Ability|EventOnEndAbility
  (params (bWasCancelled :type Boolean)))