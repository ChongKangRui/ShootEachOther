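; Gameplay ability for hold-to-aim weapon aiming, which runs Aim on activation and Unaim on input release or ability end.
; Aim switches rotation mode, applies the equipped weapon's trace and camera aim types, and adds a non-replicated Weapon.Aiming tag.
; For the local player it also sets reticle visibility and FOV, and widget-type aiming shows a reticle widget while hiding body and weapon.
; Unaim reverts these; the damage reticle offset is passed but never applied.
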(event Ability|EventActivateAbility
  (CallFunction|Aim)
  (Ability|Tasks|WaitInputRelease true
    (:OnRelease
      (CallFunction|Unaim)
      (Ability|EndAbility))))

(event Ability|EventOnEndAbility
  (params (bWasCancelled :type Boolean))
  (CallFunction|Unaim))

(fn Aim
  (bind _returnvalue (Class|SEOGameplayAbility|GetSEOCharacter))
  (bind _returnvalue_2 (Class|SEOGameplayAbility|GetEquippedWeaponInstance))
  (bind _returnvalue_3 (Class|SEOGameplayAbility|GetSEOCharacter))
  (bind _returnvalue_4 (Class|WeaponInstance|GetDefaultsWeaponData _returnvalue_2))
  (bind (_exponent _bulletbasespreadangle _aimingcameratype _aimfov _aimfovfromleftshift _tracesphereradius _tracesphereforwarddistance _aimingtracetype _reticlewidget _crosshairvisibilitywhenaiming _damageeffectoffsetwhenaiming) (Utilities|Struct|BreakWeaponData _returnvalue_4))
  ;[1 1 1] Disable reticle widget if needed
  (Utilities|FlowControl|Sequence
    (:then_0
      ;[1 1 1] Set necessary player state
      (Class|ALSCharacterBPI|BPISetRotationMode(Message) _returnvalue "NewEnumerator3")
      (Class|SGAAim|SetTraceState _aimingtracetype))
    (:then_1
      (Pawn|IsLocallyControlled
        (:True
          (CallFunction|SetReticleStat _crosshairvisibilitywhenaiming "Visible" _damageeffectoffsetwhenaiming)
          (Class|ALSCameraBPI|BPISetCameraParameter(Message) _returnvalue _aimfov))))
    (:then_2
      ;[1 1 1] Camera Aim Type Change
      (Class|ALSCameraBPI|BPISetCameraAimTypeEnum(Message) _returnvalue _aimingcameratype)
      (switch Utilities|FlowControl|Switch|SwitchonEAimCameraType _aimingcameratype
        (:UseWidgetAndHideWeaponAndPlayerBody
          (Pawn|IsLocallyControlled
            (:True
              (Class|PrimitiveComponent|SetOwnerNoSee (Variables|/Script/Engine.Character|GetMesh _returnvalue_3) true)
              (bind _returnvalue_5 (UserInterface|CreateWidget _reticlewidget (Class|ShootEachOtherCharacter|GetSEOPlayerController _returnvalue_3)))
              (bind _output_get (Variables|Default|SetAimWidget _returnvalue_5))
              (UserInterface|Viewport|AddtoViewport _output_get 0)
              (Class|WeaponBase|SetMeshOwnerCanSee (Variables|/Script/ShootEachOther.WeaponInventoryComponent|GetAttachedWeapon (Class|SEOGameplayAbility|GetWeaponInventoryComponent)) false))))))
    (:then_3
      (Ability|GameplayEffect|AddLooseGameplayTags (Components|GetOwner (Class|SEOGameplayAbility|GetSEOAbilitySystemComponent)) (GameplayTags|MakeLiteralGameplayTagContainer "(GameplayTags=((TagName=\"Weapon.Aiming\")))")))))

(fn Unaim
  (bind _returnvalue (Class|SEOGameplayAbility|GetSEOCharacter))
  (bind _aimwidget (Variables|Default|GetAimWidget))
  (Utilities|FlowControl|Sequence
    (:then_0
      (Class|ALSCharacterBPI|BPISetRotationMode(Message) _returnvalue "NewEnumerator1")
      (Class|SGAAim|SetTraceState (.NonAimingTraceType (Utilities|Struct|BreakWeaponData (Class|WeaponInstance|GetDefaultsWeaponData (Class|SEOGameplayAbility|GetEquippedWeaponInstance))))))
    (:then_1
      ;[1 1 1] Reenable reticle
      (Pawn|IsLocallyControlled
        (:True
          (CallFunction|SetReticleStat "Visible" "Visible" "(X=0.000000,Y=0.000000)")
          (Class|ALSCameraBPI|BPISetCameraParameter(Message) _returnvalue 9e+01))))
    (:then_2
      ;[1 1 1] Aim type Change
      (Class|ALSCameraBPI|BPISetCameraAimTypeEnum(Message) (Class|SEOGameplayAbility|GetSEOCharacter) "None")
      (switch Utilities|FlowControl|Switch|SwitchonEAimCameraType (.AimingCameraType (Utilities|Struct|BreakWeaponData (Class|WeaponInstance|GetDefaultsWeaponData (Class|SEOGameplayAbility|GetEquippedWeaponInstance))))
        (:UseWidgetAndHideWeaponAndPlayerBody
          (Pawn|IsLocallyControlled
            (:True
              (Class|PrimitiveComponent|SetOwnerNoSee (Variables|/Script/Engine.Character|GetMesh (Class|SEOGameplayAbility|GetSEOCharacter)) false)
              (Utilities|IsValid _aimwidget
                (:Is%20Valid
                  (Widget|RemovefromParent _aimwidget))
                (:Is%20Not%20Valid
                  _))
              (Class|WeaponBase|SetMeshOwnerCanSee (Variables|/Script/ShootEachOther.WeaponInventoryComponent|GetAttachedWeapon (Class|SEOGameplayAbility|GetWeaponInventoryComponent)) true))))))
    (:then_3
      (Ability|GameplayEffect|RemoveLooseGameplayTags (Components|GetOwner (Class|SEOGameplayAbility|GetSEOAbilitySystemComponent)) (GameplayTags|MakeLiteralGameplayTagContainer "(GameplayTags=((TagName=\"Weapon.Aiming\")))")))))

(fn SetReticleStat
  (params (AimReticleVisibility :type ESlateVisibility%20Enum :default "Visible") (DamageReticleVisibility :type ESlateVisibility%20Enum :default "Visible") (DamageReticleOffset :type Vector%202D%20Structure))
  (bind _asbp_first_person_character (Utilities|Casting|CastToBP_FirstPersonCharacter (Class|SEOGameplayAbility|GetSEOCharacter)))
  (Utilities|IsValid (Variables|/Game/Blueprint/Player/BP_FirstPersonCharacter.BP_FirstPersonCharacter_C|GetPlayerHUD _asbp_first_person_character)
    (:Is%20Valid
      (Utilities|FlowControl|Sequence
        (:then_0
          (Default|SetReticleVisibility (Variables|/Game/Blueprint/Player/BP_FirstPersonCharacter.BP_FirstPersonCharacter_C|GetPlayerHUD _asbp_first_person_character) AimReticleVisibility))
        (:then_1
          (Widget|SetVisibility (Variables|/Game/Blueprint/Widget/W_Reticle.W_Reticle_C|GetDamageReticle (Variables|/Game/Blueprint/Widget/W_PlayerHud.W_PlayerHud_C|GetW_Reticle (Variables|/Game/Blueprint/Player/BP_FirstPersonCharacter.BP_FirstPersonCharacter_C|GetPlayerHUD _asbp_first_person_character))) DamageReticleVisibility))))))