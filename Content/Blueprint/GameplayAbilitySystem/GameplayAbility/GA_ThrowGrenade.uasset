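; Gameplay ability for throwing grenades: aims while input is held, then throws on release.
; A Weapon.ThrowGrenade event during the throw montage spends ammo and, when locally controlled, detaches the attached grenade's mesh and launches it with physics along camera forward.
; When the montage ends, it spawns a replacement, or if ammo is empty clears the grenade slot and triggers Input.Slot.03, then ends the ability.
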(event Custom|Initialize%20New%20Grenade
  (bind _returnvalue (Class|WeaponInstance|InitializeforWeapon (Class|SEOGameplayAbility|GetEquippedWeaponInstance) (Class|SEOGameplayAbility|GetSEOAbilitySystemComponent) (Class|SEOGameplayAbility|GetSEOCharacter)))
  (Variables|/Script/ShootEachOther.WeaponInventoryComponent|SetAttachedWeapon (Class|SEOGameplayAbility|GetWeaponInventoryComponent) _returnvalue))

(event Custom|ThrowGrenade
  (params (GrenadeRef :type Primitive%20Component%20Object%20Reference) (ThrowVelocity :type Vector))
  (Transformation|DetachFromComponent GrenadeRef "KeepWorld" "KeepWorld" "KeepWorld" true)
  (Physics|SetSimulatePhysics GrenadeRef true)
  (Collision|SetCollisionEnabled GrenadeRef "QueryAndPhysics")
  (Collision|SetCollisionResponsetoChannel GrenadeRef "ECC_WorldStatic" "ECR_Block")
  (Collision|SetCollisionResponsetoChannel GrenadeRef "ECC_WorldDynamic" "ECR_Block")
  (Physics|SetPhysicsLinearVelocity GrenadeRef ThrowVelocity false "None"))

(event Ability|EventActivateAbility
  (bind _returnvalue (Class|SEOGameplayAbility|GetEquippedWeaponInstance))
  (bind _returnvalue_2 (Class|SEOGameplayAbility|GetEquippedWeaponInstance))
  (bind _returnvalue_3 (Class|SEOGameplayAbility|GetWeaponInventoryComponent))
  (bind _returnvalue_4 (Class|WeaponInstance|GetStatCount _returnvalue_2 "(TagName=\"Weapon.Ammo.Current\")"))
  (bind _attachedweapon (Variables|/Script/ShootEachOther.WeaponInventoryComponent|GetAttachedWeapon _returnvalue_3))
  (bind _returnvalue_5 (> _returnvalue_4 0))
  (if _returnvalue_5
    (CallFunction|Aim)
    (Ability|Tasks|WaitInputRelease true
      (:OnRelease
        (|PlayMontageandWaitProxy "None" "/Game/3rd_Party/ImportedAsset/ALS_Mixamo/Grenade_Throw_Throw_Montage.Grenade_Throw_Throw_Montage" 1.0 "None" true 1.0 0.0 false
          (:then
            (Ability|Tasks|WaitGameplayEvent "(TagName=\"Weapon.ThrowGrenade\")" (Class|SEOGameplayAbility|GetSEOCharacter) true
              (:EventReceived
                (Class|ALSCharacterBPI|BPISetRotationMode(Message) (Class|SEOGameplayAbility|GetSEOCharacter) "NewEnumerator1")
                (Class|WeaponInstance|RemoveStatCount _returnvalue "(TagName=\"Weapon.Ammo.Current\")" 1)
                (Pawn|IsLocallyControlled
                  (:True
                    (Utilities|IsValid _attachedweapon
                      (:Is%20Valid
                        (Class|WeaponBase|SetWeaponData _attachedweapon _returnvalue)
                        (CallFunction|ThrowGrenade (Actor|GetComponentbyClass _attachedweapon "/Script/Engine.StaticMeshComponent") (* (Transformation|GetActorForwardVector (Variables|/Script/Engine.PlayerController|GetPlayerCameraManager (Class|ShootEachOtherCharacter|GetSEOPlayerController (Class|SEOGameplayAbility|GetSEOCharacter)))) 1e+03)))))))))
          (:OnCompleted
            (if _returnvalue_5 :!label _label
              (CallFunction|InitializeNewGrenade)
              (else
                (Class|WeaponInventoryComponent|RemoveWeaponfromSlot (Class|SEOGameplayAbility|GetWeaponInventoryComponent) "Grenade")
                (Class|SEOAbilitySystemComponent|AbilityInputTagPressed (Class|SEOGameplayAbility|GetSEOAbilitySystemComponent) (GameplayTags|MakeLiteralGameplayTag "(TagName=\"Input.Slot.03\")"))))
            (Ability|EndAbility))
          (:OnBlendOut
            (goto _label))
          (:OnInterrupted
            (goto _label))
          (:OnCancelled
            (goto _label)))))))

(event Ability|EventOnEndAbility
  (params (bWasCancelled :type Boolean)))

(fn Aim
  (Utilities|FlowControl|Sequence
    (:then_0
      ;[1 1 1] Set necessary player state
      (Class|ALSCharacterBPI|BPISetRotationMode(Message) (Class|SEOGameplayAbility|GetSEOCharacter) "NewEnumerator3"))
    (:then_1
      (Ability|GameplayEffect|AddLooseGameplayTags (Components|GetOwner (Class|SEOGameplayAbility|GetSEOAbilitySystemComponent)) (GameplayTags|MakeLiteralGameplayTagContainer "(GameplayTags=((TagName=\"Weapon.Aiming\")))")))))

(fn SetReticleStat
  (params (AimReticleVisibility :type ESlateVisibility%20Enum :default "Visible") (DamageReticleVisibility :type ESlateVisibility%20Enum :default "Visible") (DamageReticleOffset :type Vector%202D%20Structure))
  (bind _asbp_first_person_character (Utilities|Casting|CastToBP_FirstPersonCharacter (Class|SEOGameplayAbility|GetSEOCharacter)))
  (Utilities|IsValid (Variables|/Game/Blueprint/Player/BP_FirstPersonCharacter.BP_FirstPersonCharacter_C|GetPlayerHUD _asbp_first_person_character)
    (:Is%20Valid
      (Utilities|FlowControl|Sequence
        (:then_0
          (Default|SetReticleVisibility (Variables|/Game/Blueprint/Player/BP_FirstPersonCharacter.BP_FirstPersonCharacter_C|GetPlayerHUD _asbp_first_person_character) AimReticleVisibility))
        (:then_1
          (Widget|SetVisibility (Variables|/Game/Blueprint/Widget/W_Reticle.W_Reticle_C|GetDamageReticle (Variables|/Game/Blueprint/Widget/W_PlayerHud.W_PlayerHud_C|GetW_Reticle (Variables|/Game/Blueprint/Player/BP_FirstPersonCharacter.BP_FirstPersonCharacter_C|GetPlayerHUD _asbp_first_person_character))) DamageReticleVisibility))))))