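; Background-usage character Blueprint that tints a segmented mesh by body part.
; Its construction script creates a dynamic material instance for each body-part slot, then sets every BaseColor parameter to DefaultColor.
; An outfit branch for skin, shirt, pants, shoes and gloves colors, with a solid-color option, is present but never runs.
; Event graph nodes are disabled placeholders, so the Blueprint has no runtime logic.
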(event EventBeginPlay)

(event Collision|EventActorBeginOverlap
  (params (OtherActor :type Actor%20Object%20Reference)))

(event EventTick
  (params (DeltaSeconds :type Float%20%28single-precision%29)))

(fn ConstructionScript
  (CallFunction|SetDynamicMaterials)
  (CallFunction|Set/ResetColors))

(fn SetDynamicMaterials
  (Utilities|FlowControl|Sequence
    (:then_0
      (bind _returnvalue (Rendering|Material|CreateDynamicMaterialInstance (Variables|Default|GetMesh) 2 0 "None" :!class /Script/Engine.PrimitiveComponent))
      (Variables|Default|SetHead _returnvalue)
      (bind _returnvalue_2 (Rendering|Material|CreateDynamicMaterialInstance (Variables|Default|GetMesh) 1 0 "None" :!class /Script/Engine.PrimitiveComponent))
      (Variables|Default|SetTorso _returnvalue_2)
      (bind _returnvalue_3 (Rendering|Material|CreateDynamicMaterialInstance (Variables|Default|GetMesh) 0 0 "None" :!class /Script/Engine.PrimitiveComponent))
      (Variables|Default|SetPelvis _returnvalue_3))
    (:then_1
      (bind _returnvalue_4 (Rendering|Material|CreateDynamicMaterialInstance (Variables|Default|GetMesh) 6 0 "None" :!class /Script/Engine.PrimitiveComponent))
      (Variables|Default|SetUpperLegs _returnvalue_4)
      (bind _returnvalue_5 (Rendering|Material|CreateDynamicMaterialInstance (Variables|Default|GetMesh) 7 0 "None" :!class /Script/Engine.PrimitiveComponent))
      (Variables|Default|SetLowerLegs _returnvalue_5)
      (bind _returnvalue_6 (Rendering|Material|CreateDynamicMaterialInstance (Variables|Default|GetMesh) 8 0 "None" :!class /Script/Engine.PrimitiveComponent))
      (Variables|Default|SetFeet _returnvalue_6))
    (:then_2
      (bind _returnvalue_7 (Rendering|Material|CreateDynamicMaterialInstance (Variables|Default|GetMesh) 4 0 "None" :!class /Script/Engine.PrimitiveComponent))
      (Variables|Default|SetShoulder_L _returnvalue_7)
      (bind _returnvalue_8 (Rendering|Material|CreateDynamicMaterialInstance (Variables|Default|GetMesh) 3 0 "None" :!class /Script/Engine.PrimitiveComponent))
      (Variables|Default|SetUpperArm_L _returnvalue_8)
      (bind _returnvalue_9 (Rendering|Material|CreateDynamicMaterialInstance (Variables|Default|GetMesh) 5 0 "None" :!class /Script/Engine.PrimitiveComponent))
      (Variables|Default|SetLowerArm_L _returnvalue_9)
      (bind _returnvalue_10 (Rendering|Material|CreateDynamicMaterialInstance (Variables|Default|GetMesh) 9 0 "None" :!class /Script/Engine.PrimitiveComponent))
      (Variables|Default|SetHand_L _returnvalue_10))
    (:then_3
      (bind _returnvalue_11 (Rendering|Material|CreateDynamicMaterialInstance (Variables|Default|GetMesh) 12 0 "None" :!class /Script/Engine.PrimitiveComponent))
      (Variables|Default|SetShoulder_R _returnvalue_11)
      (bind _returnvalue_12 (Rendering|Material|CreateDynamicMaterialInstance (Variables|Default|GetMesh) 11 0 "None" :!class /Script/Engine.PrimitiveComponent))
      (Variables|Default|SetUpperArm_R _returnvalue_12)
      (bind _returnvalue_13 (Rendering|Material|CreateDynamicMaterialInstance (Variables|Default|GetMesh) 13 0 "None" :!class /Script/Engine.PrimitiveComponent))
      (Variables|Default|SetLowerArm_R _returnvalue_13)
      (bind _returnvalue_14 (Rendering|Material|CreateDynamicMaterialInstance (Variables|Default|GetMesh) 14 0 "None" :!class /Script/Engine.PrimitiveComponent))
      (Variables|Default|SetHand_R _returnvalue_14))))

(fn Set/ResetColors
  (Rendering|Material|SetVectorParameterValue (Variables|Default|GetHead) "BaseColor" (Variables|Default|GetDefaultColor) :!class /Script/Engine.MaterialInstanceDynamic))