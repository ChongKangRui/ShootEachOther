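; Game state Blueprint that prints the team rosters as a debug check.
; Tick runs through a three-second Delay, and a DoOnce on the authority side limits the dump to a single pass.
; That pass loops over TeamInfo and prints each valid player's display name with its TeamID.
; The file only reads TeamInfo and contains no logic that fills it.
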(event EventBeginPlay)

(event EventTick
  (params (DeltaSeconds :type Float%20%28single-precision%29))
  (Utilities|FlowControl|Delay 3.0)
  (Networking|SwitchHasAuthority
    (:Authority
      (Utilities|FlowControl|DoOnce false
        (:Completed
          (for _array_element (Variables|Default|GetTeamInfo)
            (for _array_element_2 (.players _array_element)
              (Utilities|IsValid _array_element_2
                (:Is%20Valid
                  (Development|PrintString (Utilities|String|Append (Utilities|String|ToString(Integer) (.teamid _array_element)) "|Player=" (Utilities|GetDisplayName _array_element_2)) true true "(R=0.000000,G=0.660000,B=1.000000,A=1.000000)" 1e+01))))))))))

(fn ConstructionScript)