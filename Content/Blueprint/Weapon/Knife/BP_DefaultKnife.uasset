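; BP_DefaultKnife is a knife weapon Blueprint that is mostly a stub.
; BeginPlay calls the parent, then prints a red "meleew" debug string.
; GetMeleeTraceStart and GetMeleeTraceEnd both return zero vectors, so neither supplies a real melee trace position yet.
; Overlap and Tick events are disabled, and the construction script only calls its parent.
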(event EventBeginPlay
  (|CallParentFunction)
  (Development|PrintString "meleew" true true "(R=1.000000,G=0.000000,B=0.041046,A=1.000000)" 1e+01))

(event Collision|EventActorBeginOverlap
  (params (OtherActor :type Actor%20Object%20Reference))
  (|CallParentFunction OtherActor) ; This node is disabled and will not be called.\nDrag off pins to build functionality.
)

(event EventTick
  (params (DeltaSeconds :type Float%20%28single-precision%29))
  (|CallParentFunction DeltaSeconds) ; This node is disabled and will not be called.\nDrag off pins to build functionality.
)

(fn ConstructionScript
  (|CallParentFunction))

(fn GetMeleeTraceStart
  (return "0, 0, 0"))

(fn GetMeleeTraceEnd
  (return "0, 0, 0"))