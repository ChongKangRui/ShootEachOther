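; Weapon fire effect Blueprint that plays optional Niagara muzzle flash and tracer effects when Fire is called.
; CreateEffectInstance reuses an active attached component or spawns a new one, then flips a by-ref bool.
; That toggle feeds each system's User.Trigger to retrigger it without respawning.
; The muzzle flash gets a direction toward the first impact position, while the tracer receives the whole ImpactPositions array.
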(event Custom|Fire
  (bind _muzzleflashcomponent (Variables|Default|GetMuzzleFlashComponent))
  (bind _tracercomponent (Variables|Default|GetTracerComponent))
  (Utilities|FlowControl|Sequence
    (:then_0
      ;[1 1 1] Muzzle Flash
      (if (Variables|Default|GetEnable%20Muzzle%20Flash)
        (CallFunction|CreateEffectInstance (Variables|DefaultNiagaraSystem|GetMuzzleFlash) _muzzleflashcomponent (Variables|Trigger|GetMuzzleFlashTrigger))
        ;[1 1 1] Set Muzzle Flash Param
        (Class|NiagaraComponent|SetVariableBool _muzzleflashcomponent "User.Trigger" (Variables|Trigger|GetMuzzleFlashTrigger))
        (Niagara|SetNiagaraVariable(Vector3) _muzzleflashcomponent "User.Direction" (Math|Vector|Normalize (- (Utilities|Array|Get(acopy) (Variables|Default|GetImpact%20Positions)) (Transformation|GetActorLocation))))))
    (:then_1
      ;[1 1 1] Tracer
      (if (Variables|Default|GetEnable%20Tracer)
        (CallFunction|CreateEffectInstance (Variables|DefaultNiagaraSystem|GetTracerSystem) _tracercomponent (Variables|Trigger|GetTracerTrigger))
        ;[1 1 1] Set Tracer Param
        (Class|NiagaraComponent|SetVariableBool _tracercomponent "User.Trigger" (Variables|Trigger|GetTracerTrigger))
        (Class|NiagaraDataInterfaceArrayFunctionLibrary|SetNiagaraArrayVector _tracercomponent "User.ImpactPositions" (Variables|Default|GetImpact%20Positions))))))

(fn ConstructionScript)

(fn CreateEffectInstance
  (params (Effect :type Niagara%20System%20Object%20Reference) (Instance :type Niagara%20Component%20Object%20Reference%20%28by%20ref%29) (Triggered? :type Boolean%20%28by%20ref%29))
  (Utilities|IsValid Instance
    (:Is%20Valid
      (if (Components|Activation|IsActive Instance)
        _
        (else
          (bind _returnvalue (Niagara|SpawnSystemAttached Effect (Variables|Default|GetDefaultSceneRoot) "None" "0, 0, 0" "0, 0, 0" "SnapToTarget" true :!label _label))
          (|SetBy-RefVar Instance _returnvalue)
          (|SetBy-RefVar Triggered? false))))
    (:Is%20Not%20Valid
      (goto _label)))
  (|SetBy-RefVar Triggered? (not Triggered?))
  (return))