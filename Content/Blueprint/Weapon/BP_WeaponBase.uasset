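; Base weapon actor Blueprint, apparently for weapons used by BP_FirstPersonCharacter.
; Its construction script sets every static and skeletal mesh component to ignore all collision channels; nodes re-blocking the Camera channel are left disconnected.
; BeginPlay casts the instigator to the first-person character but does nothing further.
; DisableMeshForLocal is a stub that only prints a debug string on an always-true branch, without hiding any mesh.
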(event Custom|DisableMeshForLocal
  (if true
    (Development|PrintString "yes instigator and a player")
    (else
      (Development|PrintString "not instigator and a player"))))

(event EventBeginPlay
  (Utilities|Casting|CastToBP_FirstPersonCharacter (Game|GetInstigator)))

(event Collision|EventActorBeginOverlap
  (params (OtherActor :type Actor%20Object%20Reference)))

(event EventTick
  (params (DeltaSeconds :type Float%20%28single-precision%29)))

(fn ConstructionScript
  (for _array_element (Actor|GetComponentsByClass "/Script/Engine.StaticMeshComponent")
    (Collision|SetCollisionResponsetoAllChannels _array_element "ECR_Ignore"))
  (for _array_element_2 (Actor|GetComponentsByClass "/Script/Engine.SkeletalMeshComponent")
    (Collision|SetCollisionResponsetoAllChannels _array_element_2 "ECR_Ignore")))