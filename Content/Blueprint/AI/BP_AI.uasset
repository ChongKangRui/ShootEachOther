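; BP_AI is the bot AI controller Blueprint that starts and stops behavior tree logic for its pawn.
; StartAILogic starts the brain component if valid and runs BT_Bot, while StopAILogic stops that component's logic.
; Tick and Possess only forward to the parent class.
; An unconnected debug print compares the current target with the Blackboard "Target" value.
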(event Custom|StartAILogic
  (bind _braincomponent (Variables|Default|GetBrainComponent))
  (Utilities|IsValid _braincomponent
    (:Is%20Valid
      (AI|Logic|StartLogic _braincomponent))
    (:Is%20Not%20Valid
      _))
  (AI|RunBehaviorTree "/Game/Blueprint/AI/BT_Bot.BT_Bot"))

(event Custom|StopAI%20Logic
  (bind _braincomponent (Variables|Default|GetBrainComponent))
  (Utilities|IsValid _braincomponent
    (:Is%20Valid
      (AI|Logic|StopLogic _braincomponent ""))))

(event EventPossess
  (params (PossessedPawn :type Pawn%20Object%20Reference))
  (|CallParentFunction PossessedPawn))

(event EventTick
  (params (DeltaSeconds :type Float%20%28single-precision%29))
  (|CallParentFunction DeltaSeconds))

(fn ConstructionScript)